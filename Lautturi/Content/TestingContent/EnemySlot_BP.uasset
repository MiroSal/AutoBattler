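; EnemySlot_BP is a testing-content slot that holds an enemy character and animates its appearance.
; The NewCharacterCreated event starts a Tick-driven scale lerp that grows the slotted character from zero to full size over two seconds.
; A second function, not called in this graph, shrinks a given actor, destroys it near zero scale and requests a new character for the slot.
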(event EventBeginPlay)

(event Collision|EventActorBeginOverlap
  (params (OtherActor :type Actor%20Object%20Reference)))

(event EventTick
  (params (DeltaSeconds :type Float%20%28single-precision%29))
  (if (Variables|Default|GetStart)
    (CallFunction|NewFunction0 (Variables|Default|GetCharacterInSlot) DeltaSeconds)))

(event EventNewCharacterCreated
  (Variables|Default|SetStart true))

(fn ConstructionScript)

(fn NewFunction0
  (params (self2 :type Actor%20Object%20Reference) (A :type Float%20%28single-precision%29))
  (bind _output_get (Variables|Default|SetAlpha (+ A (Variables|Default|GetAlpha))))
  (Transformation|SetActorScale3D self2 (Math|Vector|Lerp(Vector) "0, 0, 0" "1.000000,1.000000,1.000000" (/ _output_get 2.0)))
  (if (>= (.X (Math|Vector|BreakVector (Math|Vector|Lerp(Vector) "0, 0, 0" "1.000000,1.000000,1.000000" (/ _output_get 2.0)))) 1.0)
    (Variables|Default|SetStart false)
    (Variables|Default|SetAlpha 0.0)))

(fn NewFunction1
  (params (self2 :type Actor%20Object%20Reference) (A :type Float%20%28single-precision%29))
  (bind _output_get (Variables|Default|SetAlpha (+ A (Variables|Default|GetAlpha))))
  (Transformation|SetActorScale3D self2 (Math|Vector|Lerp(Vector) "1.000000,1.000000,1.000000" "0, 0, 0" _output_get))
  (if (<= (.X (Math|Vector|BreakVector (Math|Vector|Lerp(Vector) "1.000000,1.000000,1.000000" "0, 0, 0" _output_get))) 0.1)
    (Actor|DestroyActor self2)
    (Class|BaseSlot|CreateNewCharactetoSlot)))