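; Game mode Blueprint that switches the game from a picking phase to a combat phase using level streaming.
; On BeginPlay it streams in the picking level.
; LoadCombatLevel_Event loads the level named by CombatLevel, unloads the picking level and sets a short timer by function name.
; The timer calls StartGame, which starts combat by popping the next skill action from the combat manager's queue.
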(event Custom|LoadCombatLevel_Event
  (Game|LoadStreamLevel(byName) (Utilities|String|StringToName (Variables|Default|GetCombatLevel)) true true)
  (Game|UnloadStreamLevel(byName) (Variables|Default|GetPickingLevel) true)
  (Utilities|Time|SetTimerbyFunctionName 0 "StartGame" 3.0))

(event EventBeginPlay
  (Game|LoadStreamLevel(byName) (Variables|Default|GetPickingLevel) true true))

(event EventTick
  (params (DeltaSeconds :type Float%20%28single-precision%29)))

(fn ConstructionScript)

(fn StartGame
  (bind _returnvalue (Class|LautturiGameModeBase|GetCombatManager))
  (Class|CombatManager|PopNextSkillActionfromQueue _returnvalue))