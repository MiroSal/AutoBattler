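; Test enemy Blueprint for a slot-based combat system, with placeholder attack behavior.
; Damage spawns a floating combat text widget at the enemy's projected screen position.
; Death plays a scaled explosion at the occupied slot and removes the character from it.
; An attack starts a timer by function name that calls Test, which prints a debug message and ends the attack.
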(event EventBeginPlay
  (Development|PrintString "Hello"))

(event Collision|EventActorBeginOverlap
  (params (OtherActor :type Actor%20Object%20Reference)))

(event EventTick
  (params (DeltaSeconds :type Float%20%28single-precision%29)))

(event EventAttackBlueprint
  (Utilities|Time|SetTimerbyFunctionName 0 "Test" 2.0))

(event EventOnDeath
  (Utilities|IsValid self
    (:Is%20Valid
      (bind _returnvalue (Class|EnemyBase|GetSlot))
      (Utilities|IsValid _returnvalue
        (:Is%20Valid
          (Effects|SpawnEmitteratLocation "/Game/StarterContent/Particles/P_Explosion.P_Explosion" (Transformation|GetActorLocation _returnvalue) "0, 0, 0" "2.000000,2.000000,2.000000")
          (Class|BaseSlot|RemoveCharacterfromSlot _returnvalue true))))))

(event EventDamageTaken
  (params (Amount :type Integer))
  (bind _returnvalue (UserInterface|CreateWidget "/Game/TestingContent/FloatingCombatText.FloatingCombatText_C" 0 (.ScreenPosition (Class|GameplayStatics|ProjectWorldtoScreen (Game|GetPlayerController 0) (Transformation|GetWorldLocation (Variables|Default|GetObjRoot)) false)) (Math|Conversions|ToFloat(Integer) Amount)))
  (UserInterface|Viewport|AddtoViewport _returnvalue 0))

(fn ConstructionScript)

(fn Test
  (Development|PrintString "Ënemy is attacking")
  (Class|CharacterBase|AttackEnd))