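; Skill Blueprint that heals every soul card returned by GetAllSouls when activated.
; Each card gets HealthAdd by a set amount; on success it spawns a spark emitter at the card's slot, shows stat text and refreshes its data text.
; After the loop, a timer calls Test by name a few seconds later, which prints a debug string and deactivates the skill.
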(event Custom|ReceiveBeginPlay_1)

(event Custom|ReceiveActorBeginOverlap_1
  (params (OtherActor :type Actor%20Object%20Reference)))

(event Custom|ReceiveTick_1
  (params (DeltaSeconds :type Float%20%28single-precision%29)))

(event EventActivateSkill
  (bind _addamounty (Variables|Default|GetAddAmounty))
  (bind _returnvalue (Class|SkillBase|GetAllSouls))
  (for _array_element _returnvalue
    (bind _assoul_card (Utilities|Casting|CastToSoulCard _array_element))
    (bind _returnvalue_2 (Class|SoulCard|GetSlot _assoul_card))
    (bind _returnvalue_3 (Class|SoulCard|HealthAdd _assoul_card _addamounty))
    (if _returnvalue_3
      (Effects|SpawnEmitterAttached "/Game/StarterContent/Particles/P_Sparks.P_Sparks" (Variables|/Script/Lautturi.BaseSlot|GetObjRoot _returnvalue_2) "None" (Transformation|GetWorldLocation (Variables|/Script/Lautturi.BaseSlot|GetObjRoot _returnvalue_2)) "0, 0, 0" "3.000000,3.000000,3.000000" "KeepWorldPosition")
      (bind _assoul_card_bp (Utilities|Casting|CastToSoulCard_BP _array_element))
      (Default|StatText _assoul_card_bp (Utilities|Text|ToText(String) (Utilities|String|ToString(Integer) _addamounty)) (Utilities|Text|ToText(String) (Variables|Default|GetTypeText)))
      (Class|CharacterBase|UpdateDataText _array_element)))
  (Utilities|Time|SetTimerbyFunctionName 0 "Test" 3.0))

(fn ConstructionScript)

(fn Test
  (Development|PrintString 0 "Heal All Skill")
  (Class|SkillBase|DeactivateSkill))