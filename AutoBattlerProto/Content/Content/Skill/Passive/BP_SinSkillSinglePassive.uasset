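; BP_SinSkillSinglePassive is a passive skill that adjusts the Sin of one random combat player when the owner's Sin exceeds six.
; On activation it picks from the combat player listeners and, if that character has health left, applies the amount, shows stat text and refreshes its data text.
; A three-second timer then calls EndTurn to deactivate the skill, also when the owner check fails or the target has no health.
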(event EventActivateSkill
  (bind _returnvalue (Class|SkillBase|GetCombatPlayerListeners))
  (bind _asbp_player_character (Utilities|Casting|CastToBP_PlayerCharacter (Class|SkillBase|GetOwningCharacter self))
    (:then
      (if (> (Class|CharacterBase|GetSin _asbp_player_character) 6)
        (bind _asbp_player_character_2 (Utilities|Casting|CastToBP_PlayerCharacter (Utilities|Array|Get(acopy) _returnvalue (Math|Random|RandomIntegerinRange 0 (- (Utilities|Array|Length _returnvalue) 1)))))
        (if (> (Class|CharacterBase|GetHealth _asbp_player_character_2) 0)
          (Class|CharacterBase|AdjustSin _asbp_player_character_2 (Variables|Default|GetAddAmount) false)
          (Default|StatText _asbp_player_character_2 (Utilities|Text|ToText(String) (Utilities|String|ToString(Integer) (Variables|Default|GetAddAmount))) (Utilities|Text|ToText(String) (Variables|Default|GetTypeText)) "ST_Sin")
          (Class|CharacterBase|UpdateDataText _asbp_player_character_2))))
    (:CastFailed
      _))
  (Utilities|Time|SetTimerbyFunctionName 0 "EndTurn" 3.0))

(fn EndTurn
  (Development|PrintString 0 "Sin skill Single")
  (Class|SkillBase|DeactivateSkill))