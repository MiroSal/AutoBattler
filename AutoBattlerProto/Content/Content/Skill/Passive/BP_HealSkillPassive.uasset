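; BP_HealSkillPassive is a passive combat skill that heals the player character with the lowest health.
; ActivateSkill runs Activate after an animation delay, which scans the combat player listeners and tracks the weakest one's index.
; The zero-health check tests the current weakest rather than the candidate.
; The chosen character gains AddAmount health and shows heal text, then EndTurn deactivates the skill after a short timer.
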(event Custom|Activate
  (bind _returnvalue (Class|SkillBase|GetCombatPlayerListeners))
  ;[1 1 1] Search weakest soul
  (for (_array_element _array_index) _returnvalue
    (bind _asbp_player_character (Utilities|Casting|CastToBP_PlayerCharacter _array_element))
    (bind _asbp_player_character_2 (Utilities|Casting|CastToBP_PlayerCharacter (Utilities|Array|Get(acopy) _returnvalue (Variables|Default|GetWeakestSoul))))
    (if (< (Class|CharacterBase|GetHealth _asbp_player_character) (Class|CharacterBase|GetHealth _asbp_player_character_2))
      (if (> (Class|CharacterBase|GetHealth _asbp_player_character_2) 0)
        (Variables|Default|SetWeakestSoul _array_index))))
  (bind _asbp_player_character_3 (Utilities|Casting|CastToBP_PlayerCharacter (Utilities|Array|Get(acopy) _returnvalue (Variables|Default|GetWeakestSoul)))
    (:then
      (Class|CharacterBase|AdjustHealth _asbp_player_character_3 (Variables|Default|GetAddAmount) false)
      (Default|StatText _asbp_player_character_3 (Utilities|Text|ToText(String) (Utilities|String|ToString(Integer) (Variables|Default|GetAddAmount))) (Utilities|Text|ToText(String) (Variables|Default|GetTypeText)) "ST_Heal")
      (Class|CharacterBase|UpdateDataText _asbp_player_character_3)
      (Utilities|Time|SetTimerbyFunctionName 0 "EndTurn" 3.0))
    (:CastFailed
      (CallFunction|EndTurn))))

(event EventActivateSkill
  (params (AnimDelay :type Float%20%28single-precision%29))
  (Utilities|Time|SetTimerbyEvent (delegate Custom|Activate) (Math|Float|Absolute(Float) AnimDelay)))

(fn EndTurn
  (Development|PrintString 0 (Utilities|GetDisplayName self))
  (Class|SkillBase|DeactivateSkill))