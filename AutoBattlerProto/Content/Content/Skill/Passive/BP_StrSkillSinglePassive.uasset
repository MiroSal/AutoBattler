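; Passive skill that raises the Strength of one randomly chosen player character in combat.
; ActivateSkill waits for the animation delay, then Activate picks a random combat player listener, adds the amount to its Strength, shows buff stat text and refreshes its data text.
; EndTurn runs after a short timer, or immediately if the cast fails, printing the skill's name and deactivating it.
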(event Custom|Activate
  (bind _returnvalue (Class|SkillBase|GetCombatPlayerListeners))
  (bind _asbp_player_character (Utilities|Casting|CastToBP_PlayerCharacter (Utilities|Array|Get(acopy) _returnvalue (Math|Random|RandomIntegerinRange 0 (- (Utilities|Array|Length _returnvalue) 1))))
    (:then
      (Class|CharacterBase|AdjustStr _asbp_player_character (Variables|Default|GetAddAmount) false)
      (Default|StatText _asbp_player_character (Utilities|Text|ToText(String) (Utilities|String|ToString(Integer) (Variables|Default|GetAddAmount))) (Utilities|Text|ToText(String) (Variables|Default|GetTypeText)) "ST_Buff")
      (Class|CharacterBase|UpdateDataText _asbp_player_character)
      (Utilities|Time|SetTimerbyFunctionName 0 "EndTurn" 3.0))
    (:CastFailed
      (CallFunction|EndTurn))))

(event EventActivateSkill
  (params (AnimDelay :type Float%20%28single-precision%29))
  (Utilities|Time|SetTimerbyEvent (delegate Custom|Activate) (Math|Float|Absolute(Float) AnimDelay)))

(fn EndTurn
  (Development|PrintString 0 (Utilities|GetDisplayName self))
  (Class|SkillBase|DeactivateSkill))