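; BP_BuffSkillNegativeAllPrimary is a combat skill that adjusts the Strength of every player character in combat.
; On activation it loops over the combat player listeners, adds AddAmount to Strength, shows Buff-styled stat text and refreshes each character's data text.
; A three-second timer then calls EndTurn, which prints a debug string and deactivates the skill.
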(event EventActivateSkill
  (for _array_element (Class|SkillBase|GetCombatPlayerListeners)
    (bind _asbp_player_character (Utilities|Casting|CastToBP_PlayerCharacter _array_element))
    (Class|CharacterBase|AdjustStr _asbp_player_character (Variables|Default|GetAddAmount) false)
    (Default|StatText _asbp_player_character (Utilities|Text|ToText(String) (Utilities|String|ToString(Integer) (Variables|Default|GetAddAmount))) (Utilities|Text|ToText(String) (Variables|Default|GetTypeText)) "ST_Buff")
    (Class|CharacterBase|UpdateDataText _asbp_player_character))
  (Utilities|Time|SetTimerbyFunctionName 0 "EndTurn" 3.0))

(fn EndTurn
  (Development|PrintString 0 "Buff Skill All")
  (Class|SkillBase|DeactivateSkill))