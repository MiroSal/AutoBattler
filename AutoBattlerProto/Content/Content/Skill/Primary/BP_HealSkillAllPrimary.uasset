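; BP_HealSkillAllPrimary is a primary combat skill that heals every player character in the fight.
; ActivateSkill delays Activate on a timer by the absolute animation delay.
; Activate loops over the combat player listeners, adding AddAmount to each character's health, showing heal stat text and refreshing its data text.
; A short fixed timer then calls EndTurn by name, which prints a debug string and deactivates the skill.
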(event Custom|Activate
  (for _array_element (Class|SkillBase|GetCombatPlayerListeners)
    (bind _asbp_player_character (Utilities|Casting|CastToBP_PlayerCharacter _array_element))
    (Class|CharacterBase|AdjustHealth _asbp_player_character (Variables|Default|GetAddAmount) false)
    (Default|StatText _asbp_player_character (Utilities|Text|ToText(String) (Utilities|String|ToString(Integer) (Variables|Default|GetAddAmount))) (Utilities|Text|ToText(String) (Variables|Default|GetTypeText)) "ST_Heal")
    (Class|CharacterBase|UpdateDataText _asbp_player_character))
  (Utilities|Time|SetTimerbyFunctionName 0 "EndTurn" 3.0))

(event EventActivateSkill
  (params (AnimDelay :type Float%20%28single-precision%29))
  (Utilities|Time|SetTimerbyEvent (delegate Custom|Activate) (Math|Float|Absolute(Float) AnimDelay)))

(fn EndTurn
  (Development|PrintString 0 "Heal all skill")
  (Class|SkillBase|DeactivateSkill))