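; BP_EnemySlot is an enemy slot that prepares the character it holds as new ones are created.
; After a short delay, NewCharacterCreated clears IsDead on the character's Enemy_AnimBP, skipping the first spawn via a flag.
; While the Start flag is set, Tick grows the character from zero to full scale over two seconds, then resets.
; Nothing in this graph sets Start.
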(event EventTick
  (params (DeltaSeconds :type Float%20%28single-precision%29))
  (bind _returnvalue (Class|SlotBase|GetCharacterinSlot))
  (if (Variables|Default|GetbStart)
    (bind _output_get (Variables|Default|SetAlpha (+ (Variables|Default|GetAlpha) DeltaSeconds)))
    (Utilities|IsValid _returnvalue
      (:Is%20Valid
        (Transformation|SetActorScale3D _returnvalue (Math|Vector|Lerp(Vector) "0, 0, 0" "1.000000,1.000000,1.000000" (/ _output_get 2.0)))
        (if (>= (.X (Math|Vector|BreakVector (Math|Vector|Lerp(Vector) "0, 0, 0" "1.000000,1.000000,1.000000" (/ _output_get 2.0)))) 1.0)
          (Variables|Default|SetbStart false)
          (Variables|Default|SetAlpha 0.0))))))

(event EventNewCharacterCreated
  (bind _returnvalue (Class|SlotBase|GetCharacterinSlot))
  (bind _mesh (Variables|/Script/AutoBattlerProto.CharacterBase|GetMesh _returnvalue))
  (bind _returnvalue_2 (Components|SkeletalMesh|GetAnimInstance _mesh))
  (Utilities|FlowControl|Delay 3.0)
  (if (Variables|Default|GetbIsNotFirstSpawn)
    (Utilities|IsValid _returnvalue
      (:Is%20Valid
        (Utilities|IsValid _returnvalue_2
          (:Is%20Valid
            (bind _asenemy_anim_bp (Utilities|Casting|CastToEnemy_AnimBP _returnvalue_2))
            (Variables|/Game/Content/Enemy/Enemy_AnimBP.Enemy_AnimBP_C|SetbIsDead _asenemy_anim_bp false)))))
    (else
      (Variables|Default|SetbIsNotFirstSpawn true))))

(fn ConstructionScript)