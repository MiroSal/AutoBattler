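; BP_EnemyCharacter is an enemy combatant in a slot-based, turn-based battle, showing a decal during its turn.
; Attack offsets the enemy along X and plays a montage, then a timer calls EndAttack to restore its position and call AttackEnd.
; Damage plays a montage and spawns a damage-number widget at its projected screen position; death plays a montage, then spawns an emitter at its slot.
; An older Tick-style return timer remains disconnected.
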(event EventBeginPlay
  (Rendering|SetVisibility (Variables|Default|GetDecal) false false))

(event EventStartTurn
  (Rendering|SetVisibility (Variables|Default|GetDecal) true false))

(event EventEndTurn
  (Rendering|SetVisibility (Variables|Default|GetDecal) false false))

(event EventAttack
  (bind _root (Variables|Default|GetRoot))
  (bind _returnvalue (Transformation|GetWorldLocation _root))
  (Variables|Default|SetInitialLocation (Math|Vector|MakeVector (.x _returnvalue) (.y _returnvalue) (.z _returnvalue)))
  (Transformation|SetRelativeLocation (Variables|Default|GetRoot) (Math|Vector|MakeVector (+ (.x _returnvalue) (Variables|Default|GetPositionModifier)) (.y _returnvalue) (.z _returnvalue)) false false)
  (Animation|Montage|PlayMontage (Variables|Character|GetMesh) 0
    (:then
      (Utilities|Time|SetTimerbyFunctionName 0 "EndAttack" 3.0))))

(event EventTick
  (params (DeltaSeconds :type Float%20%28single-precision%29)))

(event EventOnDeath
  (bind _returnvalue (Class|CharacterBase|GetCurrentSlot))
  (Animation|Montage|PlayMontage (Variables|Character|GetMesh) 0
    (:then
      (Utilities|IsValid self
        (:Is%20Valid
          (Utilities|IsValid _returnvalue
            (:Is%20Valid
              (Effects|SpawnEmitteratLocation 0 (Transformation|GetActorLocation _returnvalue) "0, 0, 0" "2.000000,2.000000,2.000000"))))))))

(event EventDamageTaken
  (params (Amount :type Integer))
  (Development|PrintString "enemy")
  (Animation|Montage|PlayMontage (Variables|Character|GetMesh) 0
    (:then
      (bind _returnvalue (UserInterface|CreateWidget 0 0 (.ScreenPosition (Class|GameplayStatics|ProjectWorldtoScreen (Game|GetPlayerController 0) (Transformation|GetWorldLocation (Variables|Default|GetRoot)) false)) (Math|Conversions|ToFloat(Integer) Amount)))
      (UserInterface|Viewport|AddtoViewport _returnvalue 0))))

(fn ConstructionScript)

(fn EndAttack
  (Development|PrintString "Ënemy is attacking")
  (Transformation|SetRelativeLocation (Variables|Default|GetRoot) (Variables|Default|GetInitialLocation) false false)
  (Class|CharacterBase|AttackEnd))