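; BP_PlayerCharacter is the player's turn-based combat character, handling visual feedback for turns, attacks, skills, damage and death.
; Turn events toggle an active decal, while damage and stat changes spawn floating text widgets at the projected screen position, with montages or particles.
; Attack offsets the root along X, then a timer calls EndAttack to restore the saved position and call AttackEnd.
; Skill montages are chosen by affect range.
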(event EventBeginPlay
  (Rendering|SetVisibility (Variables|Default|GetActiveDecal) false false))

(event EventSkillUsed
  (params (Skill :type Skill%20Base%20Object%20Reference))
  (bind _returnvalue (Class|SkillBase|GetAffectRange Skill))
  (bind _mesh (Variables|Character|GetMesh))
  (Development|PrintString (Utilities|String|EnumtoString _returnvalue))
  (switch Utilities|FlowControl|Switch|SwitchonEAffectRange _returnvalue
    (:AR_All
      (Animation|Montage|PlayMontage _mesh "/Game/TestingContent/Player/SkillAll_Montage.SkillAll_Montage"))
    (:AR_Single
      (Animation|Montage|PlayMontage _mesh "/Game/TestingContent/Player/SkillSingle_Montage.SkillSingle_Montage"))))

(event EventAttack
  (bind _root (Variables|Default|GetRoot))
  (bind _returnvalue (Transformation|GetWorldLocation _root))
  (Animation|Montage|PlayMontage (Variables|Character|GetMesh) "/Game/TestingContent/Player/Attack_Montage.Attack_Montage"
    (:then
      (Variables|Default|SetInitialLocation (Math|Vector|MakeVector (.x _returnvalue) (.y _returnvalue) (.z _returnvalue)))
      (Transformation|SetRelativeLocation (Variables|Default|GetRoot) (Math|Vector|MakeVector (+ (.x _returnvalue) (Variables|Default|GetPositionModifier)) (.y _returnvalue) (.z _returnvalue)) false false)
      (Utilities|Time|SetTimerbyFunctionName 0 "EndAttack" 3.0))))

(event EventTick
  (params (DeltaSeconds :type Float%20%28single-precision%29)))

(event EventOnDeath
  (Animation|Montage|PlayMontage 0 "/Game/TestingContent/Player/Death_Montage.Death_Montage"))

(event EventDamageTaken
  (params (Amount :type Integer))
  (bind _returnvalue (UserInterface|CreateWidget "/Game/TestingContent/FloatingCombatText.FloatingCombatText_C" 0 (.ScreenPosition (Class|GameplayStatics|ProjectWorldtoScreen (Game|GetPlayerController 0) (Transformation|GetWorldLocation (Variables|Default|GetRoot)) false)) (Math|Conversions|ToFloat(Integer) Amount)))
  (UserInterface|Viewport|AddtoViewport _returnvalue 0)
  (Animation|Montage|PlayMontage (Variables|Character|GetMesh) "/Game/TestingContent/Player/TakeDamage_Montage.TakeDamage_Montage"))

(event EventStartTurn
  (Rendering|SetVisibility (Variables|Default|GetActiveDecal) true false))

(event EventEndTurn
  (Rendering|SetVisibility (Variables|Default|GetActiveDecal) false false))

(fn ConstructionScript)

(fn EndAttack
  (Development|PrintString "Soul is attacking")
  (Transformation|SetRelativeLocation (Variables|Default|GetRoot) (Variables|Default|GetInitialLocation) false false)
  (Class|CharacterBase|AttackEnd))

(fn StatText
  (params (Amount :type Text) (stat :type Text) (SkillType :type ESkillType%20Enum :default "Heal"))
  (bind _returnvalue (UserInterface|CreateWidget "/Game/TestingContent/FloatingStatText.FloatingStatText_C" 0 (.ScreenPosition (Class|GameplayStatics|ProjectWorldtoScreen (Game|GetPlayerController 0) (Transformation|GetWorldLocation (Variables|Default|GetRoot)) false)) (Utilities|Text|ToText(String) (Utilities|String|Append (Utilities|String|ToString(Text) stat) (Utilities|String|ToString(Text) Amount)))))
  (UserInterface|Viewport|AddtoViewport _returnvalue 0)
  (switch Utilities|FlowControl|Switch|SwitchonESkillType SkillType
    (:ST_Heal
      (Components|Activation|Activate (Variables|Default|GetHeal_ParticleSystem) false))
    (:ST_Sin
      (Components|Activation|Activate (Variables|Default|GetSin_ParticleSystem) false))
    (:ST_Buff
      (Components|Activation|Activate (Variables|Default|GetBuff_ParticleSystem) false))))