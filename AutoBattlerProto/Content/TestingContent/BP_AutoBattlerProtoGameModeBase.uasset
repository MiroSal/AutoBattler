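; Game mode for the auto battler prototype that moves play from a picking phase to a combat phase through level streaming.
; On BeginPlay it blocking-loads the picking level.
; The LoadCombatLevel event loads the combat level, has the Soul Trial Manager destroy its trial characters, and unloads the picking level.
; It then starts a short timer that calls StartGame, which tells the Combat Manager to begin combat.
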(event Custom|LoadCombatLevel_Event
  (Game|LoadStreamLevel(byName) (Variables|Default|GetCombatLevel) true true)
  (bind _returnvalue (Class|AutoBattlerProtoGameModeBase|GetSoulTrialManager))
  (Class|SoulTrialManager|DestroyCharactersfromTrial _returnvalue)
  (Game|UnloadStreamLevel(byName) (Variables|Default|GetPickingLevel) false)
  (Utilities|Time|SetTimerbyFunctionName 0 "StartGame" 3.0))

(event EventBeginPlay
  (Game|LoadStreamLevel(byName) (Variables|Default|GetPickingLevel) true true))

(event EventTick
  (params (DeltaSeconds :type Float%20%28single-precision%29)))

(fn ConstructionScript)

(fn StartGame
  (bind _returnvalue (Class|AutoBattlerProtoGameModeBase|GetCombatManager))
  (Class|CombatManager|StartCombat _returnvalue))