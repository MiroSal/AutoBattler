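; BP_SoulCard is a Soul actor for turn-based combat, handling turn highlight, attack motion and floating feedback text.
; A decal, hidden at BeginPlay, shows between StartTurn and EndTurn.
; Attack offsets the root along X, Tick restores it after TimeToWait, and a delayed EndAttack prints a message and calls AttackEnd.
; DamageTaken and StatText spawn floating text widgets at the actor's projected screen position.
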(event EventBeginPlay
  (Rendering|SetVisibility (Variables|Default|GetDecal) false false))

(event Collision|EventActorBeginOverlap
  (params (OtherActor :type Actor%20Object%20Reference)))

(event EventAttack
  (bind _root (Variables|Default|GetRoot))
  (bind _returnvalue (Transformation|GetWorldLocation _root))
  (Variables|Default|SetInitialLocation (Math|Vector|MakeVector (.x _returnvalue) (.y _returnvalue) (.z _returnvalue)))
  (Transformation|SetRelativeLocation (Variables|Default|GetRoot) (Math|Vector|MakeVector (+ (.x _returnvalue) (Variables|Default|GetPositionModifier)) (.y _returnvalue) (.z _returnvalue)) false false)
  (Variables|Default|SetAttacking true))

(event EventDamageTaken
  (params (Amount :type Integer))
  (bind _returnvalue (UserInterface|CreateWidget "/Game/TestingContent/FloatingCombatText.FloatingCombatText_C" 0 (.ScreenPosition (Class|GameplayStatics|ProjectWorldtoScreen (Game|GetPlayerController 0) (Transformation|GetWorldLocation (Variables|Default|GetRoot)) false)) (Math|Conversions|ToFloat(Integer) Amount)))
  (UserInterface|Viewport|AddtoViewport _returnvalue 0))

(event EventEndTurn
  (Rendering|SetVisibility (Variables|Default|GetDecal) false false))

(event EventStartTurn
  (Rendering|SetVisibility (Variables|Default|GetDecal) true false))

(event EventTick
  (params (DeltaSeconds :type Float%20%28single-precision%29))
  (if (Variables|Default|GetAttacking)
    (if (> (Variables|Default|GetTimer) (Variables|Default|GetTimeToWait))
      (Transformation|SetRelativeLocation (Variables|Default|GetRoot) (Variables|Default|GetInitialLocation) false false)
      (Variables|Default|SetTimer 0.0)
      (Variables|Default|SetAttacking false)
      (Utilities|Time|SetTimerbyFunctionName 0 "EndAttack" 3.0)
      (else
        (Variables|Default|SetTimer (+ (Variables|Default|GetTimer) DeltaSeconds))))))

(fn ConstructionScript)

(fn EndAttack
  (Development|PrintString "Soul is attacking")
  (Class|CharacterBase|AttackEnd))

(fn StatText
  (params (Amount :type Text) (stat :type Text))
  (bind _returnvalue (UserInterface|CreateWidget "/Game/TestingContent/FloatingStatText.FloatingStatText_C" 0 (.ScreenPosition (Class|GameplayStatics|ProjectWorldtoScreen (Game|GetPlayerController 0) (Transformation|GetWorldLocation (Variables|Default|GetRoot)) false)) (Utilities|Text|ToText(String) (Utilities|String|Append (Utilities|String|ToString(Text) stat) (Utilities|String|ToString(Text) Amount)))))
  (UserInterface|Viewport|AddtoViewport _returnvalue 0))