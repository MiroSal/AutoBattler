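; Enemy slot actor that spawns a character on BeginPlay and animates it growing into view.
; BeginPlay calls SpawnNewCharacterToSlot, whose logic is not in this graph, and the NewCharacterCreated event raises a flag that starts the animation.
; While flagged, Tick lerps the slot character's scale from zero to full over two seconds, then clears the flag and timer for the next character.
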(event EventBeginPlay
  (Class|BaseSlot|SpawnNewCharactertoSlot))

(event EventTick
  (params (DeltaSeconds :type Float%20%28single-precision%29))
  (if (Variables|Default|GetbStart)
    (bind _output_get (Variables|Default|SetAlpha (+ (Variables|Default|GetAlpha) DeltaSeconds)))
    (Transformation|SetActorScale3D (Variables|Default|GetCharacterInSlot) (Math|Vector|Lerp(Vector) "0, 0, 0" "1.000000,1.000000,1.000000" (/ _output_get 2.0)))
    (if (>= (.X (Math|Vector|BreakVector (Math|Vector|Lerp(Vector) "0, 0, 0" "1.000000,1.000000,1.000000" (/ _output_get 2.0)))) 1.0)
      (Variables|Default|SetbStart false)
      (Variables|Default|SetAlpha 0.0))))

(event EventNewCharacterCreated
  (Variables|Default|SetbStart true))

(fn ConstructionScript)