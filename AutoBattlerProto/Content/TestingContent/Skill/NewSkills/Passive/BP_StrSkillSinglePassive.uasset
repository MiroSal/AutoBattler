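; Passive skill that buffs the Strength of one randomly chosen soul card.
; On activation it picks from all souls and, if that card has health above zero, adds the configured amount, then shows stat text and refreshes the card's data text on success.
; A dead pick is not rerolled.
; A three-second timer then calls EndTurn, which prints a debug string and deactivates the skill.
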(event EventActivateSkill
  (bind _returnvalue (Class|SkillBase|GetAllSouls))
  (bind _asbp_soul_card (Utilities|Casting|CastToBP_SoulCard (Utilities|Array|Get(acopy) _returnvalue (Math|Random|RandomIntegerinRange 0 (- (Utilities|Array|Length _returnvalue) 1))))
    (:then
      (bind _returnvalue_2 (Class|CharacterBase|GetHealth _asbp_soul_card))
      (if (> _returnvalue_2 0)
        (bind _returnvalue_3 (Class|CharacterBase|StrAdd _asbp_soul_card (Variables|Default|GetAddAmount)))
        (if _returnvalue_3
          (Default|StatText _asbp_soul_card (Utilities|Text|ToText(String) (Utilities|String|ToString(Integer) (Variables|Default|GetAddAmount))) (Utilities|Text|ToText(String) (Variables|Default|GetTypeText)))
          (Class|CharacterBase|UpdateDataText _asbp_soul_card))))
    (:CastFailed
      _))
  (Utilities|Time|SetTimerbyFunctionName 0 "EndTurn" 3.0))

(fn EndTurn
  (Development|PrintString 0 "Buff Skill Single")
  (Class|SkillBase|DeactivateSkill))