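; BP_SinSkillSinglePassive is a passive soul card skill that adds Sin to one random soul.
; It fires when the owning BP_SoulCard's Sin exceeds six, picking from all souls and applying AddAmount only if the target has health.
; A successful add shows stat text, refreshes the target's data text and starts a three-second timer to deactivate the skill.
; Failed owner, Sin or health checks also start that timer, but a failed add does not.
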(event EventActivateSkill
  (bind _asbp_soul_card (Utilities|Casting|CastToBP_SoulCard (Class|SkillBase|GetOwningCharacter self))
    (:then
      (bind _returnvalue (Class|CharacterBase|GetSin _asbp_soul_card))
      (if (> _returnvalue 6)
        (bind _returnvalue_2 (Class|SkillBase|GetAllSouls))
        (bind _asbp_soul_card_2 (Utilities|Casting|CastToBP_SoulCard (Utilities|Array|Get(acopy) _returnvalue_2 (Math|Random|RandomIntegerinRange 0 (- (Utilities|Array|Length _returnvalue_2) 1)))))
        (bind _returnvalue_3 (Class|CharacterBase|GetHealth _asbp_soul_card_2))
        (if (> _returnvalue_3 0)
          (bind _returnvalue_4 (Class|CharacterBase|SinAdd _asbp_soul_card_2 (Variables|Default|GetAddAmount)))
          (if _returnvalue_4
            (Default|StatText _asbp_soul_card_2 (Utilities|Text|ToText(String) (Utilities|String|ToString(Integer) (Variables|Default|GetAddAmount))) (Utilities|Text|ToText(String) (Variables|Default|GetTypeText)) "ST_Sin")
            (Class|CharacterBase|UpdateDataText _asbp_soul_card_2)
            (Utilities|Time|SetTimerbyFunctionName 0 "EndTurn" 3.0 :!label _label))
          (else
            (goto _label)))
        (else
          (goto _label))))
    (:CastFailed
      (goto _label))))

(fn EndTurn
  (Development|PrintString 0 "Sin skill Single")
  (Class|SkillBase|DeactivateSkill))