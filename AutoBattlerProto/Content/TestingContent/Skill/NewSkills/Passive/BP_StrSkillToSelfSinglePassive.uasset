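; BP_StrSkillToSelfSinglePassive is a passive skill that buffs the Str stat of its owning soul card.
; On activation it casts the owner to BP_SoulCard and, if Health is above zero and Sin exceeds a threshold, applies AddAmount, shows buff stat text and refreshes the card's data.
; A timer set by function name then calls Test, which prints a debug string and deactivates the skill.
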(event EventActivateSkill
  (bind _asbp_soul_card (Utilities|Casting|CastToBP_SoulCard (Class|SkillBase|GetOwningCharacter self))
    (:then
      (bind _returnvalue (Class|CharacterBase|GetHealth _asbp_soul_card))
      (if (> _returnvalue 0)
        (bind _returnvalue_2 (Class|CharacterBase|GetSin _asbp_soul_card))
        (if (> _returnvalue_2 3)
          (Class|CharacterBase|StrSet _asbp_soul_card (Variables|Default|GetAddAmount))
          (Default|StatText _asbp_soul_card (Utilities|Text|ToText(String) (Utilities|String|ToString(Integer) (Variables|Default|GetAddAmount))) (Utilities|Text|ToText(String) (Variables|Default|GetTypeText)) "ST_Buff")
          (Class|CharacterBase|UpdateDataText _asbp_soul_card))))
    (:CastFailed
      _))
  (Utilities|Time|SetTimerbyFunctionName 0 "Test" 3.0))

(fn Test
  (Development|PrintString 0 "Buff Skill Single")
  (Class|SkillBase|DeactivateSkill))