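; Passive heal skill Blueprint that targets the weakest player soul in combat.
; On activation it loops over the combat player listeners, tracking the index with lower health, switching only while the tracked character's health is above zero.
; It passes the heal amount to that character's SetHealth, shows heal stat text and refreshes its data text.
; A three-second timer then calls EndTurn, which prints a debug string and deactivates the skill.
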(event EventActivateSkill
  (bind _returnvalue (Class|SkillBase|GetCombatPlayerListeners))
  ;[1 1 1] Search weakest soul
  (for (_array_element _array_index) _returnvalue
    (bind _asbp_player_character (Utilities|Casting|CastToBP_PlayerCharacter _array_element))
    (bind _returnvalue_2 (Class|CharacterBase|GetHealth _asbp_player_character))
    (bind _asbp_player_character_2 (Utilities|Casting|CastToBP_PlayerCharacter (Utilities|Array|Get(acopy) _returnvalue (Variables|Default|GetWeakestSoul))))
    (bind _returnvalue_3 (Class|CharacterBase|GetHealth _asbp_player_character_2))
    (if (< _returnvalue_2 _returnvalue_3)
      (if (> _returnvalue_3 0)
        (Variables|Default|SetWeakestSoul _array_index))))
  (bind _asbp_player_character_3 (Utilities|Casting|CastToBP_PlayerCharacter (Utilities|Array|Get(acopy) _returnvalue (Variables|Default|GetWeakestSoul)))
    (:then
      (Class|CharacterBase|SetHealth _asbp_player_character_3 (Variables|Default|GetAddAmount))
      (Default|StatText _asbp_player_character_3 (Utilities|Text|ToText(String) (Utilities|String|ToString(Integer) (Variables|Default|GetAddAmount))) (Utilities|Text|ToText(String) (Variables|Default|GetTypeText)) "ST_Heal")
      (Class|CharacterBase|UpdateDataText _asbp_player_character_3))
    (:CastFailed
      _))
  (Utilities|Time|SetTimerbyFunctionName 0 "EndTurn" 3.0))

(fn EndTurn
  (Development|PrintString 0 "Heal Skill Single")
  (Class|SkillBase|DeactivateSkill))