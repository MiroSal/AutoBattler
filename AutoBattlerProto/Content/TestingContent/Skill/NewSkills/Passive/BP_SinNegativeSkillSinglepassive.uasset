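; Passive skill that applies SinReduce by a set amount to a randomly picked soul card.
; ActivateSkill checks health on one random soul, then re-rolls the index for the SinReduce target, so the two cards can differ.
; A failed health check or false SinReduce result starts a three-second timer to Test, which prints a debug string and deactivates the skill.
; The stat text update branch is disconnected.
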(event EventActivateSkill
  (bind _returnvalue (Class|SkillBase|GetAllSouls))
  (bind _assoul_card (Utilities|Casting|CastToSoulCard (Utilities|Array|Get(acopy) _returnvalue (Math|Random|RandomIntegerinRange 0 (- (Utilities|Array|Length _returnvalue) 1)))))
  (bind _returnvalue_2 (Class|CharacterBase|GetHealth _assoul_card))
  (if (> _returnvalue_2 0)
    (bind _asbp_soul_card (Utilities|Casting|CastToBP_SoulCard (Utilities|Array|Get(acopy) _returnvalue (Math|Random|RandomIntegerinRange 0 (- (Utilities|Array|Length _returnvalue) 1)))))
    (Class|SoulCard|GetSlot _asbp_soul_card)
    (bind _returnvalue_3 (Class|CharacterBase|SinReduce _asbp_soul_card (Variables|Default|GetAddAmounty)))
    (if (not _returnvalue_3)
      (Utilities|Time|SetTimerbyFunctionName 0 "Test" 3.0 :!label _label))
    (else
      (goto _label))))

(fn Test
  (Development|PrintString 0 "Sin skill Single")
  (Class|SkillBase|DeactivateSkill))