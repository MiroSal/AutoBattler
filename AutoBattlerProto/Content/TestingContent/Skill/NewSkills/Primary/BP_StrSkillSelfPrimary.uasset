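; A self-targeted primary skill that applies a Strength buff to the owning player character.
; On activation it passes AddAmount to the character's SetStr, shows buff stat text and refreshes the character's data text.
; A three-second timer then calls EndTurn, which prints a debug string and deactivates the skill.
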(event EventActivateSkill
  (bind _asbp_player_character (Utilities|Casting|CastToBP_PlayerCharacter (Class|SkillBase|GetOwningCharacter self))
    (:then
      (Class|CharacterBase|SetStr _asbp_player_character (Variables|Default|GetAddAmount))
      (Default|StatText _asbp_player_character (Utilities|Text|ToText(String) (Utilities|String|ToString(Integer) (Variables|Default|GetAddAmount))) (Utilities|Text|ToText(String) (Variables|Default|GetTypeText)) "ST_Buff")
      (Class|CharacterBase|UpdateDataText _asbp_player_character))
    (:CastFailed
      _))
  (Utilities|Time|SetTimerbyFunctionName 0 "EndTurn" 3.0))

(fn EndTurn
  (Development|PrintString 0 "Buff Skill Single")
  (Class|SkillBase|DeactivateSkill))