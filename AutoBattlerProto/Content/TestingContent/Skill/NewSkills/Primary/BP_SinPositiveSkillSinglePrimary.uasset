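; BP_SinPositiveSkillSinglePrimary is a primary combat skill that applies a Sin amount to a single random player character.
; On activation it picks a random combat player listener, passes AddAmount to SetSin, shows Sin stat text and refreshes that character's data text.
; A three-second timer then calls EndTurn, which prints a debug string and deactivates the skill.
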(event EventActivateSkill
  (bind _returnvalue (Class|SkillBase|GetCombatPlayerListeners))
  (bind _asbp_player_character (Utilities|Casting|CastToBP_PlayerCharacter (Utilities|Array|Get(acopy) _returnvalue (Math|Random|RandomIntegerinRange 0 (- (Utilities|Array|Length _returnvalue) 1))))
    (:then
      (Class|CharacterBase|SetSin _asbp_player_character (Variables|Default|GetAddAmount))
      (Default|StatText _asbp_player_character (Utilities|Text|ToText(String) (Utilities|String|ToString(Integer) (Variables|Default|GetAddAmount))) (Utilities|Text|ToText(String) (Variables|Default|GetTypeText)) "ST_Sin")
      (Class|CharacterBase|UpdateDataText _asbp_player_character))
    (:CastFailed
      _))
  (Utilities|Time|SetTimerbyFunctionName 0 "EndTurn" 3.0))

(fn EndTurn
  (Development|PrintString 0 "Sin Skill Single")
  (Class|SkillBase|DeactivateSkill))