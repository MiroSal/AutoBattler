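; Primary skill Blueprint that heals every soul card returned by GetAllSouls.
; On activation it casts each soul to BP_SoulCard and adds a configurable health amount.
; Cards where the add succeeds show stat text with the amount and type label, then refresh their data text.
; A timer then calls EndTurn by name after a short delay, which prints a debug string and deactivates the skill.
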(event EventActivateSkill
  (bind _returnvalue (Class|SkillBase|GetAllSouls))
  (for _array_element _returnvalue
    (bind _asbp_soul_card (Utilities|Casting|CastToBP_SoulCard _array_element))
    (bind _returnvalue_2 (Class|SoulCard|HealthAdd _asbp_soul_card (Variables|Default|GetAddAmount)))
    (if _returnvalue_2
      (Default|StatText _asbp_soul_card (Utilities|Text|ToText(String) (Utilities|String|ToString(Integer) (Variables|Default|GetAddAmount))) (Utilities|Text|ToText(String) (Variables|Default|GetTypeText)))
      (Class|CharacterBase|UpdateDataText _asbp_soul_card)))
  (Utilities|Time|SetTimerbyFunctionName 0 "EndTurn" 3.0))

(fn EndTurn
  (Development|PrintString 0 "Heal all skill")
  (Class|SkillBase|DeactivateSkill))